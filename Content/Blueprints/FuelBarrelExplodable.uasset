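; A fuel barrel actor that explodes when its Health component reports death.
; On death it calls Explode on its Explodable component with its Sphere, spawns an explosion particle emitter at its location and rotation, then destroys itself.
; Health tracking and explosion behavior are delegated to those components, leaving the Blueprint as event glue with no active BeginPlay, overlap or Tick logic.
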(event `self.Health.OnDeath`
  (`ExplodableComponent.Explode` (`self.Explodable`) (`self.Sphere`))
  (`GameplayStatics.SpawnEmitterAtLocation` "/Game/Particle/Explosion.Explosion" (`self.K2_GetActorLocation`) (`self.K2_GetActorRotation`))
  (`self.K2_DestroyActor`))

(fn `UserConstructionScript`
  (`parent.UserConstructionScript`))