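; Networked player unit Blueprint that fires a hitscan attack and can be killed.
; Attack input runs a short camera-forward debug line trace locally, also via a server event for clients, damaging any DamageableComponent on the hit actor.
; A locally controlled unit creates a Player_HUD on BeginPlay and links it to its ShieldedHealth component.
; ShieldedHealth's death event destroys the actor and prints a kill message.
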(event `ServerAttack`
  ;[1 1 1] LMB to Shoot
  (`self.Attack` :!label _label))

(event `InputAction|Attack`
  (params (Key :type "Key Structure"))
  ;[1 1 1] LMB to Shoot
  (:`Pressed`
    (`/Engine/EditorBlueprintResources/ActorMacros.Switch Has Authority`
      (:`Authority`
        (goto _label))
      (:`Remote`
        (`self.ServerAttack`)
        (goto _label)))))

(event `self.ShieldedHealth.OnDeath`
  (`self.K2_DestroyActor`)
  (`KismetSystemLibrary.PrintString` "Player Killed" true true (struct :`R` 1.0 :`G` 0.376235 :`A` 1.0)))

(event `self.ReceiveTick`
  (params (DeltaSeconds :type "Float (single-precision)")))

(event `self.ReceiveBeginPlay`
  (if (`self.IsLocallyControlled`)
    (bind _asplayer_controller (cast `PlayerController` (`self.GetController`)))
    (bind _returnvalue (`|CreateWidget` "/Game/Widget/Player_HUD.Player_HUD_C" _asplayer_controller))
    (`UserWidget.AddToViewport` _returnvalue 0)
    (set `/Game/Widget/Player_HUD.LinkedShieldedHealthComponent` (`self.ShieldedHealth`) _returnvalue)))

(fn `Attack`
  (bind _camera (`self.Camera`))
  (bind _returnvalue (`SceneComponent.K2_GetComponentLocation` _camera))
  (bind _outhit (`KismetSystemLibrary.LineTraceSingle` :`Start` _returnvalue :`End` (+ _returnvalue (* (`KismetMathLibrary.GetForwardVector` (`SceneComponent.K2_GetComponentRotation` _camera)) 1500.0)) :`TraceChannel` "TraceTypeQuery1" :`DrawDebugType` "ForDuration" :`TraceColor` (struct :`G` 0.956624 :`B` 1.0 :`A` 1.0) :`DrawTime` 1.0))
  (bind (_bblockinghit _binitialoverlap _time _distance _location _impactpoint _normal _impactnormal _physmat _hitactor) (`GameplayStatics.BreakHitResult` _outhit))
  (if (`KismetSystemLibrary.IsValid` _hitactor)
    (bind _returnvalue_2 (`self.GetComponentByClass` _hitactor "/Script/StationCaptured.DamageableComponent"))
    (if (`KismetSystemLibrary.IsValid` _returnvalue_2)
      (`DamageableComponent.Damage` _returnvalue_2 (`self.Damage`))
      (else
        (`KismetSystemLibrary.PrintString` "Hit sth without health")))
    (else
      (`KismetSystemLibrary.PrintString` "Nothing Hit"))))

(fn `UserConstructionScript`)