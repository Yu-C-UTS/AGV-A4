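; LaserBeam is an AI-folder actor that acts as a short-lived damaging laser shot.
; It destroys itself after a brief delay from BeginPlay, or earlier when it overlaps a valid actor on the authority.
; That authority-only overlap applies its Damage value through the other actor's DamageableComponent if present, and destroys the beam whether or not one is found.
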(event `self.ReceiveBeginPlay`
  (`KismetSystemLibrary.Delay` 2.0)
  (`self.K2_DestroyActor`))

(event `self.ReceiveActorBeginOverlap`
  (params (OtherActor :type "Actor Object Reference"))
  (bind _returnvalue (`self.GetComponentByClass` OtherActor "/Script/StationCaptured.DamageableComponent"))
  (`/Engine/EditorBlueprintResources/StandardMacros.IsValid` OtherActor
    (:`Is Valid`
      (`/Engine/EditorBlueprintResources/ActorMacros.Switch Has Authority`
        (:`Authority`
          (`/Engine/EditorBlueprintResources/StandardMacros.IsValid` _returnvalue
            (:`Is Valid`
              (`DamageableComponent.Damage` _returnvalue (`self.Damage`))
              (`self.K2_DestroyActor`))
            (:`Is Not Valid`
              (`self.K2_DestroyActor`))))))))

(event `self.Box.OnComponentBeginOverlap`
  (params (OverlappedComponent :type "PrimitiveComponent Object Reference") (OtherActor :type "Actor Object Reference") (OtherComp :type "PrimitiveComponent Object Reference") (OtherBodyIndex :type Integer) (bFromSweep :type Boolean) (SweepResult :type "HitResult Structure (by ref)")))

(fn `UserConstructionScript`)