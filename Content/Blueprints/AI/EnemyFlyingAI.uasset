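; Flying enemy AI that chases and attacks players, falls back to allies or its hive, and dies in a blood burst.
; Tick turns the whole actor toward the local player for its health widget, then branches on sight: engage, delayed ally teleport, or hive teleport, healing and random retargeting.
; Attacks line-trace forward, ignoring fellow flyers, to hit DamageableComponents.
; Retargeting quits the game when no valid player is found; Patrol is unwired.
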(event `self.ReceiveBeginPlay`
  ;[1 1 1] Health Component Ref for AI_HealthHUD
  (bind _asai_health_hud (cast `/Game/Widget/AI_HealthHUD` (`WidgetComponent.GetUserWidgetObject` (`self.Health Widget`))))
  (set `/Game/Widget/AI_HealthHUD.LinkedHealthComponent` (`self.Health1`) _asai_health_hud))

(event `self.ReceiveTick`
  (params (DeltaSeconds :type "Float (single-precision)"))
  (bind _returnvalue (`ActorComponent.GetOwner` (`self.Health Widget`)))
  (`|ExecutionSequence`
    (:`then_0`
      ;[1 1 1] Make HealthWidget Face Player
      (bind _outactors (`GameplayStatics.GetAllActorsOfClass` "/Script/StationCaptured.PlayerUnitCore"))
      (for _array_element _outactors
        (if (`self.IsLocallyControlled` _array_element)
          (`self.K2_SetActorRotation` _returnvalue (`KismetMathLibrary.FindLookAtRotation` (`self.K2_GetActorLocation` _returnvalue) (`self.K2_GetActorLocation` _array_element)) false)
          (break))))
    (:`then_1`
      (bind _returnvalue_2 (`self.CanSeePlayer`))
      (if _returnvalue_2
        ;[1 1 1] Engage
        (`self.LookAtPlayer`)
        (`self.ChasePlayer`)
        (`KismetSystemLibrary.Delay` 2.0)
        (`self.Attack`)
        (else
          ;[1 1 1] Rally
          (bind _returnvalue_3 (`self.IsRally`))
          (if _returnvalue_3
            (`KismetSystemLibrary.Delay` 2.0)
            (`self.TeleportToAlly`)
            (else
              ;[1 1 1] Hive
              (`self.TeleportToHive`)
              (`self.Healing`)
              (`self.GetOtherPlayer`))))))))

(event `self.Health1.OnDeath`
  ;[1 1 1] OnDeath
  (`GameplayStatics.SpawnEmitterAtLocation` "/Game/Particle/Blood.Blood" (`self.K2_GetActorLocation`) (`self.K2_GetActorRotation`))
  (`self.K2_DestroyActor`))

(fn `Attack`
  (bind _sphere (`self.Sphere`))
  (bind _returnvalue (`SceneComponent.K2_GetComponentLocation` _sphere))
  (bind _outactors (`GameplayStatics.GetAllActorsOfClass` "EnemyFlyingAI_C"))
  (bind _outhit (`KismetSystemLibrary.LineTraceSingle` _returnvalue (+ _returnvalue (* (`KismetMathLibrary.GetForwardVector` (`SceneComponent.K2_GetComponentRotation` _sphere)) 1250.0)) "TraceTypeQuery1" false _outactors "ForDuration" true (struct :`R` 1.0 :`A` 1.0) (struct :`G` 1.0 :`A` 1.0) 1.0))
  (bind (_bblockinghit _binitialoverlap _time _distance _location _impactpoint _normal _impactnormal _physmat _hitactor) (`GameplayStatics.BreakHitResult` _outhit))
  (if (`KismetSystemLibrary.IsValid` _hitactor)
    (bind _returnvalue_2 (`self.GetComponentByClass` _hitactor "/Script/StationCaptured.DamageableComponent"))
    (if (`KismetSystemLibrary.IsValid` _returnvalue_2)
      (`DamageableComponent.Damage` _returnvalue_2 (`self.Damage`))
      (else
        (`KismetSystemLibrary.PrintString` "AI hit sth without health" true true (struct :`R` 1.0 :`B` 0.014468 :`A` 1.0))))
    (else
      (`KismetSystemLibrary.PrintString` "AI Hit Nothing" true true (struct :`R` 1.0 :`B` 0.014468 :`A` 1.0)))))

(fn `GetOtherPlayer`
  (bind _outactors (`GameplayStatics.GetAllActorsOfClass` "/Script/StationCaptured.PlayerUnitCore"))
  (bind _output (`|GetArrayItem` _outactors (`KismetMathLibrary.RandomIntegerInRange` 0 (`KismetArrayLibrary.Array_LastIndex` _outactors))))
  (`/Engine/EditorBlueprintResources/StandardMacros.IsValid` _output
    (:`Is Valid`
      (set `self.UnitToChase` _output))
    (:`Is Not Valid`
      (`KismetSystemLibrary.PrintString` "All Player Dead")
      (`KismetSystemLibrary.QuitGame` null "Quit"))))

(fn `Healing`
  (bind _health1 (`self.Health1`))
  (bind _currenthealth (`HealthComponent.CurrentHealth` _health1))
  (if (< _currenthealth 100.0)
    (set `HealthComponent.CurrentHealth` (+ _currenthealth 1.0) _health1)))

(fn `UserConstructionScript`)