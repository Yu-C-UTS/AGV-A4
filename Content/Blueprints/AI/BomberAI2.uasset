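; Suicide bomber enemy AI that chases player units and explodes when within trigger range.
; Each Tick picks a behavior by priority: engage a visible player, rally with allies, or patrol while slowly regenerating health, with random retargeting in the latter two.
; Death from the Health component calls MulticastDeath to explode, spawn effects and destroy the actor.
; Its health widget links to that component and rotates toward the locally controlled player.
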(event `self.ReceiveBeginPlay`
  ;[1 1 1] Health Component Ref for AI_HealthHUD
  (bind _asai_health_hud (cast `/Game/Widget/AI_HealthHUD` (`WidgetComponent.GetUserWidgetObject` (`self.Health Widget`))))
  (set `/Game/Widget/AI_HealthHUD.LinkedHealthComponent` (`self.Health`) _asai_health_hud))

(event `self.ReceiveActorBeginOverlap`
  (params (OtherActor :type "Actor Object Reference")))

(event `self.ReceiveTick`
  (params (DeltaSeconds :type "Float (single-precision)"))
  (`|ExecutionSequence`
    (:`then_0`
      ;[1 1 1] Make HealthWidget Face Player
      (bind _outactors (`GameplayStatics.GetAllActorsOfClass` "/Script/StationCaptured.PlayerUnitCore"))
      (for _array_element _outactors
        (if (`self.IsLocallyControlled` _array_element)
          (`SceneComponent.K2_SetWorldRotation` (`self.Health Widget`) (`KismetMathLibrary.FindLookAtRotation` (`self.K2_GetActorLocation` (`ActorComponent.GetOwner` (`self.Health Widget`))) (`self.K2_GetActorLocation` _array_element)) false false)
          (break))))
    (:`then_1`
      (bind _returnvalue (`self.CanSeePlayer`))
      (if _returnvalue
        ;[1 1 1] Engage
        (`self.LookAtPlayer`)
        (`self.ChasePlayer`)
        (`self.SuicideBombing`)
        (else
          ;[1 1 1] Rally
          (bind _returnvalue_2 (`self.IsRally`))
          (if _returnvalue_2
            (`self.GatherWithAlly`)
            (`self.Get OtherPlayer`)
            (else
              ;[1 1 1] Scan and Patrol
              (`self.Patrol`)
              (`self.Healing`)
              (`self.Get OtherPlayer`))))))))

(event `self.Health.OnDeath`
  ;[1 1 1] OnDeath
  (`self.MulticastDeath`))

(event `MulticastDeath`
  ;[1 1 1] OnDeath
  (`ExplodableComponent.Explode` (`self.Explodable`) (`self.Sphere`))
  (`GameplayStatics.SpawnEmitterAtLocation` "/Game/Particle/Explosion.Explosion" (`self.K2_GetActorLocation`) (`self.K2_GetActorRotation`))
  (`self.K2_DestroyActor`)
  (set `self.bCanSeePlayer` false))

(fn `Get OtherPlayer`
  (bind _outactors (`GameplayStatics.GetAllActorsOfClass` "/Script/StationCaptured.PlayerUnitCore"))
  (bind _output (`|GetArrayItem` _outactors (`KismetMathLibrary.RandomIntegerInRange` 0 (`KismetArrayLibrary.Array_LastIndex` _outactors))))
  (`/Engine/EditorBlueprintResources/StandardMacros.IsValid` _output
    (:`Is Valid`
      (set `self.UnitToChase` _output))))

(fn `Healing`
  (bind _health (`self.Health`))
  (bind _currenthealth (`HealthComponent.CurrentHealth` _health))
  (if (< _currenthealth 100.0)
    (set `HealthComponent.CurrentHealth` (+ _currenthealth 0.1) _health)))

(fn `SuicideBombing`
  (if (< (`self.GetDistanceTo` (`self.UnitToChase`)) (`self.ExplodeTriggerDistance`))
    (`ExplodableComponent.Explode` (`self.Explodable`) (`self.Sphere`))
    (`GameplayStatics.SpawnEmitterAtLocation` "/Game/Particle/Explosion.Explosion" (`self.K2_GetActorLocation`) (`self.K2_GetActorRotation`))
    (`self.K2_DestroyActor`)
    (set `self.bCanSeePlayer` false)))

(fn `UserConstructionScript`)